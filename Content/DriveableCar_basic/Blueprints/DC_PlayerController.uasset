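; Player controller for the driveable car game that switches the player between an on-foot pawn and a hatchback car.
; Interact triggers the car's enter/exit event when entry is allowed or the player is not in the stored pawn.
; Helper functions handle possession and pawn visibility, returning the pawn at the car's left door.
; It also hides map text by VR tag on BeginPlay and can look up the LapTrigger by name.
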(event EventBeginPlay
  (Class|HeadMountedDisplayFunctionLibrary|SetTrackingOrigin "Eye")
  (bind _asdc_game_mode (Utilities|Casting|CastToDC_GameMode (Game|GetGameMode)))
  ;[1 1 1] Show Correct Text on Map
  (if (Variables|/Game/DriveableCar_basic/Blueprints/DC_GameMode.DC_GameMode_C|Getis_vr_enabled _asdc_game_mode)
    (bind _outactors (Actor|GetAllActorsOfClass "/Script/Engine.TextRenderActor"))
    (for _array_element _outactors
      (if (Components|ComponentHasTag (Variables|/Script/Engine.TextRenderActor|GetTextRender _array_element) "NO_VR")
        (Rendering|SetActorHiddenInGame _array_element true)))
    (else
      (bind _outactors_2 (Actor|GetAllActorsOfClass "/Script/Engine.TextRenderActor"))
      (for _array_element_2 _outactors_2
        (if (Components|ComponentHasTag (Variables|/Script/Engine.TextRenderActor|GetTextRender _array_element_2) "VR")
          (Rendering|SetActorHiddenInGame _array_element_2 true))))))

(event Input|ActionEvents|InputActionInteract
  (params (Key :type Key%20Structure))
  (:Pressed
    (if (Variables|Default|GetCanEnterCar)
      (bind _ashatchback_bp_base (Utilities|Casting|CastToHatchback_BP_Base (Variables|Default|GetCarReference)))
      (Default|CEEnterExitCar _ashatchback_bp_base)
      (elif (not (== (Game|Player|GetPlayerPawn 0) (Variables|Default|GetPawnRefernce)))
        (bind _ashatchback_bp_base_2 (Utilities|Casting|CastToHatchback_BP_Base (Variables|Default|GetCarReference)))
        (Default|CEEnterExitCar _ashatchback_bp_base_2)))))

(fn ConstructionScript)

(fn HidePawn
  (bind _pawnrefernce (Variables|Default|GetPawnRefernce))
  (Rendering|SetActorHiddenInGame _pawnrefernce true)
  (Collision|SetActorEnableCollision _pawnrefernce false))

(fn ShowPawn
  (bind _pawnrefernce (Variables|Default|GetPawnRefernce))
  (Rendering|SetActorHiddenInGame _pawnrefernce false)
  (Collision|SetActorEnableCollision _pawnrefernce true)
  (bind _ashatchback_bp_base (Utilities|Casting|CastToHatchback_BP_Base (Variables|Default|GetCarReference)))
  (Transformation|SetActorLocation (Variables|Default|GetPawnRefernce) (Transformation|GetWorldLocation (Variables|/Game/DriveableCar_basic/Blueprints/Vehicles/Hatchback_BP_Base.Hatchback_BP_Base_C|GetLeftDoor _ashatchback_bp_base)) false true))

(fn PossesCar
  (Pawn|Possess self (Variables|Default|GetCarReference)))

(fn PossesPawn
  (Pawn|Possess self (Variables|Default|GetPawnRefernce))
  (CallFunction|ShowPawn))

(fn SetLapTrigger
  (bind _outactors (Actor|GetAllActorsOfClass "/Script/Engine.TriggerBase"))
  (bind _array_element (Utilities|Array|ForEachLoopwithBreak _outactors :!label _label)
    (:LoopBody
      (if (Utilities|Enum|Equal(Enum) (Utilities|GetObjectName _array_element) "LapTrigger")
        (Variables|Default|SetLapTrigger _array_element)
        (goto _label Break)))
    (:Completed
      (return))))