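; DC_GameMode is the game mode for the driveable car project, choosing the player's on-foot pawn at startup.
; After a short BeginPlay delay it checks whether a head-mounted display is enabled.
; In VR it replaces the default pawn with a VR character at the same location and possesses it.
; Either way, it stores the active character as the pawn reference on DC_PlayerController.
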(event EventBeginPlay
  (bind _returnvalue (Game|Player|GetPlayerPawn 0))
  ;[1 1 1] Spawn VR Character
  (Utilities|FlowControl|Delay 0.05)
  (bind _output_get (Variables|Default|Setis_vr_enabled (Class|HeadMountedDisplayFunctionLibrary|IsHeadMountedDisplayEnabled)))
  (if _output_get
    (bind _output_get_2 (Variables|Default|SetPlayerStartLocation (Transformation|GetActorLocation _returnvalue)))
    (Actor|DestroyActor _returnvalue)
    (bind _returnvalue_2 (Game|SpawnActorfromClass "/Game/DriveableCar_basic/Blueprints/VRCharacter.VRCharacter_C" (Math|Transform|MakeTransform _output_get_2 "0, 0, 0" "1,1,1") "Undefined" 0 0))
    (Pawn|Possess (Game|GetPlayerController 0) _returnvalue_2)
    (bind _asdc_player_controller (Utilities|Casting|CastToDC_PlayerController (Game|GetPlayerController 0)))
    (Variables|/Game/DriveableCar_basic/Blueprints/DC_PlayerController.DC_PlayerController_C|SetPawnRefernce _asdc_player_controller _returnvalue_2)
    (else
      (bind _asdc_player_controller_2 (Utilities|Casting|CastToDC_PlayerController (Game|GetPlayerController 0)))
      (Variables|/Game/DriveableCar_basic/Blueprints/DC_PlayerController.DC_PlayerController_C|SetPawnRefernce _asdc_player_controller_2 (Game|GetPlayerCharacter 0)))))

(event EventTick
  (params (DeltaSeconds :type Float%20%28single-precision%29))
  ;[1 1 1] Spawn VR Character
)

(fn ConstructionScript)