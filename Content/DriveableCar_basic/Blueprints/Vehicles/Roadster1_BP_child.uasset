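; Roadster car Blueprint that bridges simulated vehicle sensors and external driving control, using Simulink-flagged messages for all but lidar.
; On BeginPlay it binds lidar, IMU, GPS and GPS ground-truth events, whose data is serialized and pushed through per-sensor senders.
; Received control bytes are deserialized and applied through SendControls only outside manual drive mode.
; BeginPlay also adds a camera widget to the viewport.
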(event Custom|OnIMUAvailable
  (params (IMUData :type IMU%20Message%20Structure%20%28by%20ref%29))
  (bind _returnvalue (Class|MessageSerializerComponent|SerializeIMUMessage (Variables|Default|GetMessageSerializer) IMUData true))
  (bind _returnvalue_2 (Class|TazioVehicle|GetIMUSender))
  (Utilities|IsValid _returnvalue_2
    (:Is%20Valid
      (Class|UDPSender|SendData _returnvalue_2 _returnvalue))))

(event Custom|OnDataReceived
  (params (Data :type Array%20of%20Bytes))
  ;[1 1 1] Control received
  (if (not (Class|TazioVehicle|IsManualDriveMode))
    (bind _returnvalue (Class|MessageSerializerComponent|DeserializeControlMessage (Variables|Default|GetMessageSerializer) Data true))
    (Class|TazioVehicle|SendControls _returnvalue)))

(event Custom|OnLidarAvailable
  (params (LidarScan :type Lidar%20Message%20Structure%20%28by%20ref%29))
  ;[1 1 1] Serialize and send to perception board
  (bind _returnvalue (Class|MessageSerializerComponent|SerializeLidarMessage (Variables|Default|GetMessageSerializer) LidarScan false))
  (bind _returnvalue_2 (Class|TazioVehicle|GetLidarSender))
  (Utilities|IsValid _returnvalue_2
    (:Is%20Valid
      (Class|UDPSender|SendData _returnvalue_2 _returnvalue))))

(event Custom|OnGPSTruthAvailable
  (params (GPSTruthData :type Odometry%20Message%20Structure%20%28by%20ref%29))
  (bind _returnvalue (Class|MessageSerializerComponent|SerializeOdometryMessage (Variables|Default|GetMessageSerializer) GPSTruthData true))
  (bind _returnvalue_2 (Class|TazioVehicle|GetGPSTruthSender))
  (Class|UDPSender|SendData _returnvalue_2 _returnvalue))

(event Custom|OnGPSAvailable
  (params (GPSData :type Odometry%20Message%20Structure%20%28by%20ref%29))
  (bind _returnvalue (Class|MessageSerializerComponent|SerializeOdometryMessage (Variables|Default|GetMessageSerializer) GPSData true))
  (bind _returnvalue_2 (Class|TazioVehicle|GetGPSSender))
  (Class|UDPSender|SendData _returnvalue_2 _returnvalue))

(event EventBeginPlay
  (EventDispatchers|AssignOnLidarAvailable (Variables|Default|GetLidar) (delegate Custom|OnLidarAvailable))
  (bind _returnvalue (Class|TazioVehicle|GetControlReceiver))
  (EventDispatchers|AssignOnDataReceived _returnvalue (delegate Custom|OnDataReceived))
  (EventDispatchers|AssignOnIMUAvailable (Variables|Default|GetIMU) (delegate Custom|OnIMUAvailable))
  (bind _returnvalue_2 (UserInterface|CreateWidget "/Game/CameraWidget.CameraWidget_C" (Game|GetPlayerController 0)))
  (UserInterface|Viewport|AddtoViewport _returnvalue_2 0)
  (EventDispatchers|BindEventtoOnGPSAvailable (Variables|Default|GetGPS) (delegate Custom|OnGPSAvailable))
  (EventDispatchers|AssignOnGPSTruthAvailable (Variables|Default|GetGPS) (delegate Custom|OnGPSTruthAvailable)))

(event EventTick
  (params (DeltaSeconds :type Float%20%28single-precision%29)))

(fn ConstructionScript
  (|CallParentFunction))