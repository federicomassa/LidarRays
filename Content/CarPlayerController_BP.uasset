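; Player controller for a car that owns the car data HUD and the lidar on/off state.
; On BeginPlay it enables lidar, then creates the CarDataUI widget and adds it to the viewport.
; The LidarToggle input flips the ActivateLidar flag, and incoming lidar scan events are forwarded straight to the widget.
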(event Custom|OnLidarDataAvailable
  (params (LidarScan :type Lidar%20Message%20Object%20Reference))
  (Default|OnLidarDataAvailable (Variables|Default|GetCarDataUI) LidarScan))

(event EventBeginPlay
  (Variables|Default|SetActivateLidar true)
  (bind _returnvalue (UserInterface|CreateWidget "/Game/CarDataUI_BP.CarDataUI_BP_C" self))
  (UserInterface|Viewport|AddtoViewport _returnvalue 0)
  (Variables|Default|SetCarDataUI _returnvalue))

(event EventTick
  (params (DeltaSeconds :type Float%20%28single-precision%29)))

(event Input|ActionEvents|InputActionLidarToggle
  (params (Key :type Key%20Structure))
  (:Pressed
    (Variables|Default|SetActivateLidar (not (Variables|Default|GetActivateLidar)))))

(fn ConstructionScript)