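; Game instance that holds the simulator's session configuration and persists it between runs in a "Config" save slot.
; On Init it loads the existing SaveGame_BP and copies its fields into its own variables, or creates a new save object if none exists.
; On Shutdown it copies the variables back and writes the slot.
; Settings cover level, vehicle, sensor, control and race-control network endpoints, contestants, and replay and track-map paths.
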(event EventInit
  (bind _returnvalue (SaveGame|DoesSaveGameExist "Config"))
  (if _returnvalue
    (bind _returnvalue_2 (SaveGame|LoadGamefromSlot "Config"))
    (bind _assave_game_bp (Utilities|Casting|CastToSaveGame_BP _returnvalue_2))
    (Variables|Default|SetSaveGame _assave_game_bp)
    (CallFunction|LoadConfiguration)
    (else
      (bind _returnvalue_3 (SaveGame|CreateSaveGameObject "/Game/Menu/SaveGame_BP.SaveGame_BP_C"))
      (Variables|Default|SetSaveGame _returnvalue_3))))

(event EventShutdown
  (CallFunction|SaveConfiguration)
  (SaveGame|SaveGametoSlot (Variables|Default|GetSaveGame) "Config"))

(fn LoadConfiguration
  (bind _savegame (Variables|Default|GetSaveGame))
  (bind _savegame_2 (Variables|Default|GetSaveGame))
  (bind _savegame_3 (Variables|Default|GetSaveGame))
  (bind _savegame_4 (Variables|Default|GetSaveGame))
  (bind _savegame_5 (Variables|Default|GetSaveGame))
  (bind _savegame_6 (Variables|Default|GetSaveGame))
  (bind _savegame_7 (Variables|Default|GetSaveGame))
  (Variables|Default|SetLevelName (Variables|/Game/Menu/SaveGame_BP.SaveGame_BP_C|GetLevelName _savegame_2))
  (Variables|Default|SetVehicleModel (Variables|/Game/Menu/SaveGame_BP.SaveGame_BP_C|GetVehicleModel _savegame_2))
  (Variables|Default|SetLidarSendIP (Variables|/Game/Menu/SaveGame_BP.SaveGame_BP_C|GetLidarSendIP _savegame_3))
  (Variables|Default|SetLidarPort (Variables|/Game/Menu/SaveGame_BP.SaveGame_BP_C|GetLidarPort _savegame_3))
  (Variables|Default|SetGPSSendIP (Variables|/Game/Menu/SaveGame_BP.SaveGame_BP_C|GetGPSSendIP _savegame_4))
  (Variables|Default|SetGPSPort (Variables|/Game/Menu/SaveGame_BP.SaveGame_BP_C|GetGPSPort _savegame_4))
  (Variables|Default|SetGPSTruthSendIP (Variables|/Game/Menu/SaveGame_BP.SaveGame_BP_C|GetGPSTruthSendIP _savegame_5))
  (Variables|Default|SetGPSTruthPort (Variables|/Game/Menu/SaveGame_BP.SaveGame_BP_C|GetGPSTruthPort _savegame_5))
  (Variables|Default|SetIMUSendIP (Variables|/Game/Menu/SaveGame_BP.SaveGame_BP_C|GetIMUSendIP _savegame_6))
  (Variables|Default|SetIMUPort (Variables|/Game/Menu/SaveGame_BP.SaveGame_BP_C|GetIMUPort _savegame_6))
  (Variables|Default|SetControlReceiveIP (Variables|/Game/Menu/SaveGame_BP.SaveGame_BP_C|GetControlReceiveIP _savegame_7))
  (Variables|Default|SetControlPort (Variables|/Game/Menu/SaveGame_BP.SaveGame_BP_C|GetControlPort _savegame_7))
  (Variables|Default|SetContestants (Variables|/Game/Menu/SaveGame_BP.SaveGame_BP_C|GetContestants (Variables|Default|GetSaveGame)))
  (Variables|Default|SetReplayTrajectoryPath (Variables|/Game/Menu/SaveGame_BP.SaveGame_BP_C|GetReplayTrajectoryPath (Variables|Default|GetSaveGame)))
  (Variables|Default|SetOpponentStateSendIP (Variables|/Game/Menu/SaveGame_BP.SaveGame_BP_C|GetOpponentStateSendIP (Variables|Default|GetSaveGame)))
  (Variables|Default|SetOpponentStatePort (Variables|/Game/Menu/SaveGame_BP.SaveGame_BP_C|GetOpponentStatePort (Variables|Default|GetSaveGame)))
  (Variables|Default|SetTrackMapFilePath (Variables|/Game/Menu/SaveGame_BP.SaveGame_BP_C|GetTrackMapFilePath (Variables|Default|GetSaveGame)))
  (Variables|Default|SetRaceControlSendIP (Variables|/Game/Menu/SaveGame_BP.SaveGame_BP_C|GetRaceControlSendIP _savegame))
  (Variables|Default|SetRaceControlPort (Variables|/Game/Menu/SaveGame_BP.SaveGame_BP_C|GetRaceControlPort _savegame)))

(fn SaveConfiguration
  (bind _savegame (Variables|Default|GetSaveGame))
  (Variables|/Game/Menu/SaveGame_BP.SaveGame_BP_C|SetLevelName (Variables|Default|GetSaveGame) (Variables|Default|GetLevelName))
  (Variables|/Game/Menu/SaveGame_BP.SaveGame_BP_C|SetVehicleModel (Variables|Default|GetSaveGame) (Variables|Default|GetVehicleModel))
  (Variables|/Game/Menu/SaveGame_BP.SaveGame_BP_C|SetLidarSendIP (Variables|Default|GetSaveGame) (Variables|Default|GetLidarSendIP))
  (Variables|/Game/Menu/SaveGame_BP.SaveGame_BP_C|SetLidarPort (Variables|Default|GetSaveGame) (Variables|Default|GetLidarPort))
  (Variables|/Game/Menu/SaveGame_BP.SaveGame_BP_C|SetGPSSendIP (Variables|Default|GetSaveGame) (Variables|Default|GetGPSSendIP))
  (Variables|/Game/Menu/SaveGame_BP.SaveGame_BP_C|SetGPSPort (Variables|Default|GetSaveGame) (Variables|Default|GetGPSPort))
  (Variables|/Game/Menu/SaveGame_BP.SaveGame_BP_C|SetGPSTruthSendIP (Variables|Default|GetSaveGame) (Variables|Default|GetGPSTruthSendIP))
  (Variables|/Game/Menu/SaveGame_BP.SaveGame_BP_C|SetGPSTruthPort (Variables|Default|GetSaveGame) (Variables|Default|GetGPSTruthPort))
  (Variables|/Game/Menu/SaveGame_BP.SaveGame_BP_C|SetIMUSendIP (Variables|Default|GetSaveGame) (Variables|Default|GetIMUSendIP))
  (Variables|/Game/Menu/SaveGame_BP.SaveGame_BP_C|SetIMUPort (Variables|Default|GetSaveGame) (Variables|Default|GetIMUPort))
  (Variables|/Game/Menu/SaveGame_BP.SaveGame_BP_C|SetControlReceiveIP (Variables|Default|GetSaveGame) (Variables|Default|GetControlReceiveIP))
  (Variables|/Game/Menu/SaveGame_BP.SaveGame_BP_C|SetControlPort (Variables|Default|GetSaveGame) (Variables|Default|GetControlPort))
  (Variables|/Game/Menu/SaveGame_BP.SaveGame_BP_C|SetContestants (Variables|Default|GetSaveGame) (Variables|Default|GetContestants))
  (Variables|/Game/Menu/SaveGame_BP.SaveGame_BP_C|SetReplayTrajectoryPath (Variables|Default|GetSaveGame) (Variables|Default|GetReplayTrajectoryPath))
  (Variables|/Game/Menu/SaveGame_BP.SaveGame_BP_C|SetOpponentStateSendIP (Variables|Default|GetSaveGame) (Variables|Default|GetOpponentStateSendIP))
  (Variables|/Game/Menu/SaveGame_BP.SaveGame_BP_C|SetOpponentStatePort (Variables|Default|GetSaveGame) (Variables|Default|GetOpponentStatePort))
  (Variables|/Game/Menu/SaveGame_BP.SaveGame_BP_C|SetTrackMapFilePath (Variables|Default|GetSaveGame) (Variables|Default|GetTrackMapFilePath))
  (Variables|/Game/Menu/SaveGame_BP.SaveGame_BP_C|SetRaceControlSendIP _savegame (Variables|Default|GetRaceControlSendIP))
  (Variables|/Game/Menu/SaveGame_BP.SaveGame_BP_C|SetRaceControlPort _savegame (Variables|Default|GetRaceControlPort)))