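; VehiclePawn_BP is a simulated vehicle pawn that links to an external perception board over UDP and can be driven by received control messages.
; Each Lidar scan is serialized and sent through the UDP sender, then passed to CarPlayerController_BP.
; Incoming UDP data is deserialized outside manual drive mode, mapping linear X to forward movement and negated angular Z to steering.
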(event Custom|OnLidarAvailable
  (params (LidarScan :type Lidar%20Message%20Object%20Reference))
  ;[1 1 1] Serialize and send to perception board
  (bind _returnvalue (Class|MessageSerializerComponent|SerializeLidarMessage (Variables|Default|GetMessageSerializer) LidarScan))
  (bind _returnvalue_2 (Class|VehicleTestPawn|GetUDPSender))
  (Class|UDPSender|SendData _returnvalue_2 _returnvalue)
  ;[1 1 1] Notify player controller
  (bind _ascar_player_controller_bp (Utilities|Casting|CastToCarPlayerController_BP (Game|GetPlayerController 0)))
  (Default|OnLidarDataAvailable _ascar_player_controller_bp LidarScan))

(event Custom|OnControlReceived
  (params (Data :type Array%20of%20Bytes))
  ;[1 1 1] Control received
  (if (not (Class|VehicleTestPawn|IsManualDriveMode))
    (bind _returnvalue (Class|MessageSerializerComponent|DeserializeControlMessage (Variables|Default|GetMessageSerializer) Data))
    (Class|VehicleTestPawn|MoveForward (.X (Math|Vector|BreakVector (Class|TwistMessage|GetLinear _returnvalue))))
    (Class|VehicleTestPawn|MoveRight (* (.Z (Math|Vector|BreakVector (Class|TwistMessage|GetAngular _returnvalue))) -1.0))))

(event EventBeginPlay
  (EventDispatchers|AssignOnLidarAvailable (Variables|Default|GetLidar) (delegate Custom|OnLidarAvailable))
  (bind _returnvalue (Class|VehicleTestPawn|GetUDPReceiver))
  (EventDispatchers|BindEventtoOnDataReceived _returnvalue (delegate Custom|OnControlReceived)))

(event Collision|EventActorBeginOverlap
  (params (OtherActor :type Actor%20Object%20Reference)))

(fn ConstructionScript)